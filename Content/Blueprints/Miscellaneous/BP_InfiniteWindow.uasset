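; BP_InfiniteWindow is a portal window whose plane shows a live view from its linked Other window.
; On BeginPlay it feeds a viewport-sized render target from Other's scene capture into a dynamic M_Portal material.
; Each post-update tick moves that capture to mirror the player camera relative to both windows, resizing the target with the viewport.
; It sets a clip plane base and normal on its own capture but leaves clipping disabled.
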(event `self.ReceiveBeginPlay`
  (bind (_returnvalue_x _returnvalue_y) (`KismetMathLibrary.BreakVector2D` (`WidgetLayoutLibrary.GetViewportSize`)))
  (`self.SetTickGroup` "TG_PostUpdateWork")
  (bind _returnvalue (`KismetMaterialLibrary.CreateDynamicMaterialInstance` "/Game/Materials/M_Portal.M_Portal"))
  (bind _output_get (set `self.Material` _returnvalue))
  (`PrimitiveComponent.SetMaterial` (`self.Plane`) 0 _output_get)
  (bind _returnvalue_2 (`KismetRenderingLibrary.CreateRenderTarget2D` (`KismetMathLibrary.FTrunc` _returnvalue_x) (`KismetMathLibrary.FTrunc` _returnvalue_y)))
  (bind _output_get_2 (set `self.RenderTarget` _returnvalue_2))
  (`MaterialInstanceDynamic.SetTextureParameterValue` (`self.Material`) "Texture" _output_get_2)
  (set `SceneCaptureComponent2D.TextureTarget` (`self.RenderTarget`) (`/Game/Blueprints/Miscellaneous/BP_InfiniteWindow.CameraPortal` (`self.Other`)))
  (`self.SetClipPlanes`))

(event `self.ReceiveTick`
  (params (DeltaSeconds :type "Float (single-precision)"))
  (`self.UpdateSceneCapture`)
  (`self.CheckViewportSize`))

(fn `CheckViewportSize`
  (bind (_returnvalue_x _returnvalue_y) (`KismetMathLibrary.BreakVector2D` (`WidgetLayoutLibrary.GetViewportSize`)))
  (bind _rendertarget (`self.RenderTarget`))
  (bind (_x _y) (`KismetMathLibrary.BreakVector2D` (`WidgetLayoutLibrary.GetViewportSize`)))
  (if (not (and (== _x (`TextureRenderTarget2D.SizeX` _rendertarget)) (== _y (`TextureRenderTarget2D.SizeY` _rendertarget))))
    (`KismetRenderingLibrary.ResizeRenderTarget2D` (`self.RenderTarget`) (`KismetMathLibrary.FTrunc` _returnvalue_x) (`KismetMathLibrary.FTrunc` _returnvalue_y))))

(fn `SetClipPlanes`
  (bind _cameraportal (`self.CameraPortal`))
  (`/Engine/EditorBlueprintResources/StandardMacros.IsValid` (`self.Other`)
    (:`Is Valid`
      (set `SceneCaptureComponent2D.bEnableClipPlane` false _cameraportal)
      (set `SceneCaptureComponent2D.ClipPlaneBase` (+ (`SceneComponent.K2_GetComponentLocation` (`self.Plane`)) (* (`SceneComponent.GetForwardVector` (`self.Forward`)) -3.0)) _cameraportal)
      (set `SceneCaptureComponent2D.ClipPlaneNormal` (`SceneComponent.GetForwardVector` (`self.Forward`)) _cameraportal))))

(fn `UpdateSceneCapture`
  (bind _returnvalue (`self.GetTransform`))
  (bind _returnvalue_2 (`self.GetTransform` (`self.Other`)))
  (bind (_x _y _z) (`KismetMathLibrary.BreakRotIntoAxes` (`SceneComponent.K2_GetComponentRotation` (`PlayerCameraManager.TransformComponent` (`GameplayStatics.GetPlayerCameraManager` 0)))))
  (`SceneComponent.K2_SetWorldLocationAndRotation` (`/Game/Blueprints/Miscellaneous/BP_InfiniteWindow.CameraPortal` (`self.Other`)) (`KismetMathLibrary.TransformLocation` (`self.GetTransform` (`self.Other`)) (`KismetMathLibrary.InverseTransformLocation` (`KismetMathLibrary.MakeTransform` (.location (`self.GetTransform`)) (.rotation (`self.GetTransform`)) (`KismetMathLibrary.MakeVector` (* (.x (.scale (`self.GetTransform`))) -1.0) (* (.y (.scale (`self.GetTransform`))) -1.0) (.z (.scale (`self.GetTransform`))))) (`SceneComponent.K2_GetComponentLocation` (`PlayerCameraManager.TransformComponent` (`GameplayStatics.GetPlayerCameraManager` 0))))) (`KismetMathLibrary.MakeRotationFromAxes` (`KismetMathLibrary.TransformDirection` _returnvalue_2 (`KismetMathLibrary.MirrorVectorByNormal` (`KismetMathLibrary.MirrorVectorByNormal` (`KismetMathLibrary.InverseTransformDirection` _returnvalue _x) (1.0 0.0 0.0)) (0.0 1.0 0.0))) (`KismetMathLibrary.TransformDirection` _returnvalue_2 (`KismetMathLibrary.MirrorVectorByNormal` (`KismetMathLibrary.MirrorVectorByNormal` (`KismetMathLibrary.InverseTransformDirection` _returnvalue _y) (1.0 0.0 0.0)) (0.0 1.0 0.0))) (`KismetMathLibrary.TransformDirection` _returnvalue_2 (`KismetMathLibrary.MirrorVectorByNormal` (`KismetMathLibrary.MirrorVectorByNormal` (`KismetMathLibrary.InverseTransformDirection` _returnvalue _z) (1.0 0.0 0.0)) (0.0 1.0 0.0)))) false false))

(fn `UserConstructionScript`)